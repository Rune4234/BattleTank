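; Tank pawn Blueprint that wires up the tank's barrel and turret and handles player aim and fire input.
; On BeginPlay it registers the Barrel and Turret components through setter functions.
; Aim axes orbit the camera rig, with yaw on an azimuth gimbal and local pitch on the spring arm, keeping the two rotations separate.
; The TankFire press calls Fire, whose logic is defined outside these graphs.
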(event `self.ReceiveBeginPlay`
  (`self.SetBarrelReference` (`self.Barrel`))
  (`self.SetTurretReference` (`self.Turret`)))

(event `InputAxis|AimAzimuth`
  (params (AxisValue :type "Float (single-precision)"))
  ;[1 1 1] Input Binding
  (`SceneComponent.K2_AddRelativeRotation` (`self.Azimuth Gimbal`) (`KismetMathLibrary.MakeRotator` 0.0 0.0 AxisValue) false false))

(event `InputAxis|AimElevation`
  (params (AxisValue :type "Float (single-precision)"))
  ;[1 1 1] Input Binding
  (`SceneComponent.K2_AddLocalRotation` (`self.SpringArm`) (`KismetMathLibrary.MakeRotator` 0.0 AxisValue) false false))

(event `InputAction|TankFire`
  (params (Key :type "Key Structure"))
  ;[1 1 1] Input Binding
  (:`Pressed`
    (`self.Fire`)))

(fn `UserConstructionScript`)